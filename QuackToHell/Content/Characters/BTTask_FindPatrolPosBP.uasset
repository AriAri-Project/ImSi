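; Behavior tree task that picks a random patrol destination for a QNonPlayer NPC.
; If the NPC is talking, it focuses the controller on the player pawn and succeeds without choosing a new point.
; Otherwise it writes a random reachable point within SearchRadius of the pawn to LocationKey and finishes with the query's success flag.
; A failed cast to QNonPlayer leaves the task unfinished.
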(event `self.ReceiveExecuteAI`
  (params (OwnerController :type "AIController Object Reference") (ControlledPawn :type "Pawn Object Reference"))
  (bind (_randomlocation _returnvalue) (`NavigationSystemV1.K2_GetRandomReachablePointInRadius` (`Actor.K2_GetActorLocation` ControlledPawn) (`self.SearchRadius`) null null))
  (bind _asqnon_player (cast `QNonPlayer` ControlledPawn))
  (if (`QNonPlayer.bIsTalking` _asqnon_player)
    (`AIController.K2_SetFocus` OwnerController (`GameplayStatics.GetPlayerPawn` 0))
    (`self.FinishExecute` true)
    (else
      (`BTFunctionLibrary.SetBlackboardValueAsVector` (`self.LocationKey`) _randomlocation)
      (`self.FinishExecute` _returnvalue))))